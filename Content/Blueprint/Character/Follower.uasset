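; Follower character Blueprint that displays a level name on an attached widget component.
; On BeginPlay it gets the level name from the actor itself and writes it into the description text of its GsEditorWidgetBP widget.
; Each Tick it requests a rotation facing the player camera and applies it to the widget when successful, so the label acts as a billboard.
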(event `self.ReceiveBeginPlay`
  (bind _returnvalue (`LevelUtile.GetLevelNameFromActor` self))
  (bind _asgs_editor_widget_bp (cast `/Game/BlueprintEditor/Terrain/GsEditorWidgetBP` (`WidgetComponent.GetUserWidgetObject` (`self.Widget`))))
  (`TextBlock.SetText` (`GsEditorWidget._DescriptionText` _asgs_editor_widget_bp) (`KismetTextLibrary.Conv_NameToText` _returnvalue)))

(event `self.ReceiveTick`
  (params (DeltaSeconds :type "Float (single-precision)"))
  (bind _widget (`self.Widget`))
  (bind _returnvalue (`JavascriptLibrary.Actor_GetWorld` self))
  (bind (_out_rot _returnvalue_2) (`UIUtile.TryGetRotationForFacePlayerCamera` _returnvalue (`SceneComponent.K2_GetComponentLocation` _widget)))
  (if _returnvalue_2
    (`SceneComponent.K2_SetWorldRotation` _widget _out_rot false false)))

(event `self.Mesh.OnAnimInitialized`)

(fn `UserConstructionScript`)