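; TestNavCreatorBP is a test pawn that displays a level name on a widget and logs its lifecycle events.
; On BeginPlay it writes the level name obtained from itself into the DescriptionText of its GsEditorWidgetBP widget.
; Each Tick rotates the widget component to face the player camera.
; Reset, unpossess, end-play and destroy events print a label and the actor's name for debugging.
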(event `self.ReceiveBeginPlay`
  (bind _returnvalue (`LevelUtile.GetLevelNameFromActor` self))
  (bind _asgs_editor_widget_bp (cast `/Game/BlueprintEditor/Terrain/GsEditorWidgetBP` (`WidgetComponent.GetUserWidgetObject` (`self.Widget`))))
  (`TextBlock.SetText` (`GsEditorWidget._DescriptionText` _asgs_editor_widget_bp) (`KismetTextLibrary.Conv_NameToText` _returnvalue)))

(event `self.ReceiveTick`
  (params (DeltaSeconds :type "Float (single-precision)"))
  (bind _widget (`self.Widget`))
  (bind _returnvalue (`JavascriptLibrary.Actor_GetWorld` self))
  (bind (_out_rot _returnvalue_2) (`UIUtile.TryGetRotationForFacePlayerCamera` _returnvalue (`SceneComponent.K2_GetComponentLocation` _widget)))
  (if _returnvalue_2
    (`SceneComponent.K2_SetWorldRotation` _widget _out_rot false false)))

(event `self.K2_OnReset`
  (`KismetSystemLibrary.PrintString` "Reset" true true (struct :`G` 0.282915 :`B` 1.0 :`A` 1.0))
  (bind _returnvalue (`JavascriptLibrary.GetName` self))
  (`KismetSystemLibrary.PrintString` _returnvalue))

(event `self.ReceiveUnpossessed`
  (params (OldController :type "Controller Object Reference"))
  (`KismetSystemLibrary.PrintString` "Unposssed" true true (struct :`R` 1.0 :`G` 0.068094 :`A` 1.0))
  (bind _returnvalue (`JavascriptLibrary.GetName` self))
  (`KismetSystemLibrary.PrintString` _returnvalue))

(event `self.ReceiveEndPlay`
  (params (EndPlayReason :type "EEndPlayReason Enum" :default "Destroyed"))
  (`KismetSystemLibrary.PrintString` "End Play")
  (bind _returnvalue (`JavascriptLibrary.GetName` self))
  (`KismetSystemLibrary.PrintString` _returnvalue))

(event `self.ReceiveDestroyed`
  (`KismetSystemLibrary.PrintString` "Destory" true true (struct :`R` 0.616688 :`G` 1.0 :`A` 1.0))
  (bind _returnvalue (`JavascriptLibrary.GetName` self))
  (`KismetSystemLibrary.PrintString` _returnvalue))

(fn `UserConstructionScript`)