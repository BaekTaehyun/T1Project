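; GsEditorTerrainZoneBP is a terrain zone actor, apparently for editor use, that builds its visual from an array of points.
; The construction script initializes the points, destroys existing components, then adds a root-attached pillar and plane component per point.
; It registers pillars by index and planes without one, then calls Draw once all are created.
; The event graph holds only inactive stub events.
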(fn `UserConstructionScript`
  (bind __pointarray (`self._PointArray`))
  (`self.InitPoints`)
  (`KismetSystemLibrary.PrintString` "Point : ")
  (`KismetSystemLibrary.PrintString` (`KismetStringLibrary.Conv_IntToString` 0))
  (`self.DestoryAllComponents`)
  (`|ExecutionSequence`
    (:`then_0`
      (for (_ _array_index) __pointarray
        (bind _returnvalue (`AddComponent|NODE_AddGsEditorTerrainPillarComp-2`))
        (`SceneComponent.K2_AttachToComponent` _returnvalue (`self._Root`) "None" "KeepRelative" "KeepRelative" "KeepRelative" true)
        (`self.RegisterPillar` _returnvalue _array_index)))
    (:`then_1`
      (for _ __pointarray
        (bind _returnvalue_2 (`AddComponent|NODE_AddGsEditorTerrainPlaneComp-0`))
        (`SceneComponent.K2_AttachToComponent` _returnvalue_2 (`self._Root`) "None" "KeepRelative" "KeepRelative" "KeepRelative" true)
        (`self.RegisterPlane` _returnvalue_2)))
    (:`then_2`
      (`self.Draw`))))