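; LevelIndicatorBP is a prop that labels itself with the name of the level it gets from its own actor.
; The construction script stores that name as the Description string, then calls the widget text and position refresh functions, so the label updates on construction.
; BeginPlay repeats the name lookup and text refresh but leaves the position as is.
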(event `self.ReceiveBeginPlay`
  (bind _returnvalue (`LevelUtile.GetLevelNameFromActor` self))
  (set `self._Description` (`KismetStringLibrary.Conv_NameToString` _returnvalue))
  (`self.InvalideWidgetText`))

(fn `UserConstructionScript`
  (bind _returnvalue (`LevelUtile.GetLevelNameFromActor` self))
  (set `self._Description` (`KismetStringLibrary.Conv_NameToString` _returnvalue))
  (`self.InvalideWidgetText`)
  (`self.InvalideWidgetPosition`))